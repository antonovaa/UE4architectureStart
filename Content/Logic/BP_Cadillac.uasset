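; BP_Cadillac moves a convoy of skeletal meshes along a looping spline.
; The construction script spawns the meshes at even intervals and stores each one's spline distance in a map.
; Each tick advances them by Velocity and eases each forward toward its neighbors' midpoint, wrapping at spline length.
; After Startmonitoring, proximity to OtherCadollacs' elements overrides Velocity and the easing divisor with fixed values, never restored here.
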(event `self.ReceiveBeginPlay`)

(event `self.ReceiveTick`
  (params (DeltaSeconds :type "Float (single-precision)"))
  (for (_array_element _array_index) (`self.Elements`)
    (`self.CalculateNextPoint` _array_index (* DeltaSeconds (`self.velocity`)) _array_element)))

(event `CalculateNextPoint`
  (params (numberPoint :type Integer) (constShift :type "Float (double-precision)") (Target :type "SceneComponent Object Reference"))
  (bind _spline (`self.Spline`))
  (bind _currentpositiondistance (`self.currentPositionDistance`))
  (bind _currentdist (`self.currentDist`))
  (bind _lenght (`self.lenght`))
  (bind (_value _returnvalue) (`BlueprintMapLibrary.Map_Find` (`self.StartLocation`) (- numberPoint 1)))
  (bind (_value_2 _returnvalue_2) (`BlueprintMapLibrary.Map_Find` (`self.StartLocation`) numberPoint))
  (bind (_value_3 _returnvalue_3) (`BlueprintMapLibrary.Map_Find` (`self.StartLocation`) (+ numberPoint 1)))
  ;[1 1 1] current Elemet
  (set `self.currentDist` _value_2)
  (if _returnvalue_2
    ;[1 1 1] next Element
    (if _returnvalue_3
      (set `self.nextDist` _value_3)
      (else
        (set `self.nextDist` (`BlueprintMapLibrary.Map_Find` (`self.StartLocation`)))))
    ;[1 1 1] previous Element
    (if _returnvalue
      (set `self.previousDist` _value)
      (else
        (set `self.previousDist` (`BlueprintMapLibrary.Map_Find` (`self.StartLocation`) (`self.CountCadillacs`)))))
    ;[1 1 1] step-by-step))
    (if (not (>= (`self.nextDist`) (`self.currentDist`)))
      (set `self.nextDist` (+ (`self.nextDist`) (`self.lenght`))))
    (if (not (>= (`self.currentDist`) (`self.previousDist`)))
      (set `self.currentDist` (+ (`self.currentDist`) (`self.lenght`))))
    (if (not (>= (`self.nextDist`) (`self.previousDist`)))
      (set `self.previousDist` (- (`self.previousDist`) (`self.lenght`))))
    ;[1 1 1] in avverage points
    ;;[1 1 1] offset
    (set `self.Target` (mod (/ (+ (`self.nextDist`) (`self.previousDist`)) 2.0) _lenght))
    (set `self.currentDist` (mod (`self.currentDist`) _lenght))
    (if (<= (`self.Target`) (`self.currentDist`))
      (set `self.Target` _currentdist))
    ;;[1 1 1] check other Elements
    (if (`self.isStrart`)
      (for _array_element (`/Game/Logic/BP_Cadillac.Elements` (`self.otherCadollacs`))
        (if (<= (`KismetMathLibrary.VSize` (- (`SplineComponent.GetLocationAtDistanceAlongSpline` (`self.Spline`) (`self.currentPositionDistance`) "World") (`SceneComponent.K2_GetComponentLocation` _array_element))) (`self.maxDistance`))
          (set `self.speedBetween` 1000.0)
          (set `self.velocity` 1.0))))
    (bind _output_get (set `self.currentPositionDistance` (+ constShift (+ _currentdist (/ (- (`self.Target`) _currentdist) (`self.speedBetween`))))))
    (`BlueprintMapLibrary.Map_Add` (`self.StartLocation`) numberPoint _output_get)
    (`SceneComponent.K2_SetRelativeLocationAndRotation` Target (`SplineComponent.GetLocationAtDistanceAlongSpline` _spline _currentpositiondistance "Local") (`SplineComponent.GetRotationAtDistanceAlongSpline` _spline _currentpositiondistance "Local") false false)))

(event `Start monitoring`
  (set `self.isStrart` true))

(fn `UserConstructionScript`
  (bind _spline (`self.Spline`))
  (for _index (range (+ (`self.CountCadillacs`) 1))
    (bind _returnvalue (* _index (`self.StartPositionLenght`)))
    (`BlueprintMapLibrary.Map_Add` (`self.StartLocation`) _index _returnvalue)
    (bind _returnvalue_2 (`AddComponent|NODE_AddSkeletalMeshComponent-2` :`RelativeTransform` (`KismetMathLibrary.MakeTransform` (`SplineComponent.GetLocationAtDistanceAlongSpline` _spline _returnvalue "Local") (`SplineComponent.GetRotationAtDistanceAlongSpline` _spline _returnvalue "Local"))))
    (`KismetArrayLibrary.Array_Add` (`self.Elements`) _returnvalue_2))
  (set `self.lenght` (`SplineComponent.GetSplineLength` _spline)))